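; BP_Checkpoint is a checkpoint actor that records a respawn point for the third-person character.
; On BeginPlay it creates a dynamic instance of M_Checkpoint on the Checkpoint mesh.
; When a BP_ThirdPersonCharacter overlaps the Box, it writes the actor's location to the character's LastCheckpoint, sets IsActive and turns the material's ColorBase green.
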(event OnComponentBeginOverlap(Box)
  (params (OverlappedComponent :type Primitive%20Component%20Object%20Reference) (OtherActor :type Actor%20Object%20Reference) (OtherComp :type Primitive%20Component%20Object%20Reference) (OtherBodyIndex :type Integer) (bFromSweep :type Boolean) (SweepResult :type Hit%20Result%20Structure%20%28by%20ref%29))
  (bind _asbp_third_person_character (Utilities|Casting|CastToBP_ThirdPersonCharacter OtherActor))
  (Variables|/Game/ThirdPerson/Blueprints/BP_ThirdPersonCharacter.BP_ThirdPersonCharacter_C|SetLastCheckpoint _asbp_third_person_character (Transformation|GetActorLocation))
  (Variables|Default|SetbIsActive true)
  (if (Variables|Default|GetbIsActive)
    (Rendering|Material|SetVectorParameterValue (Variables|Default|GetDynamicMat) "ColorBase" "(R=0.128676,G=1.000000,B=0.004110,A=1.000000)" :!class /Script/Engine.MaterialInstanceDynamic)))

(event EventBeginPlay
  (bind _returnvalue (Rendering|Material|CreateDynamicMaterialInstance (Variables|Default|Getcheckpoint) 0 "/Game/Materials/M_Checkpoint.M_Checkpoint" "None" :!class /Script/Engine.PrimitiveComponent))
  (bind _output_get (Variables|Default|SetDynamicMat _returnvalue))
  (Rendering|Material|SetMaterial (Variables|Default|Getcheckpoint) 0 _output_get))

(event Collision|EventActorBeginOverlap
  (params (OtherActor :type Actor%20Object%20Reference)))

(event EventTick
  (params (DeltaSeconds :type Float%20%28single-precision%29)))

(fn ConstructionScript)