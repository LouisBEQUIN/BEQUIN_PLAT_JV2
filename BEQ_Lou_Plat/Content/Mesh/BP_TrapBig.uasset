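; BP_TrapBig is a moving trap that damages the third-person character on contact.
; On BeginPlay a timeline lerps it from its start location along its forward vector by Distance, without sweeping.
; Each time the timeline finishes, it waits briefly and reverses from the end, so after the first outward move only the return stroke repeats.
; Box overlaps with BP_ThirdPersonCharacter call TakeDammage with a fixed amount.
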(event OnComponentBeginOverlap(Box)
  (params (OverlappedComponent :type Primitive%20Component%20Object%20Reference) (OtherActor :type Actor%20Object%20Reference) (OtherComp :type Primitive%20Component%20Object%20Reference) (OtherBodyIndex :type Integer) (bFromSweep :type Boolean) (SweepResult :type Hit%20Result%20Structure%20%28by%20ref%29))
  (bind _asbp_third_person_character (Utilities|Casting|CastToBP_ThirdPersonCharacter OtherActor))
  (Default|TakeDammage _asbp_third_person_character 2e+01))

(event EventBeginPlay
  (Variables|Default|SetStartLocation (Transformation|GetActorLocation))
  (bind _newtrack_0 (Timeline|Timeline Play)
    (:Update
      (Transformation|SetActorLocation (Math|Vector|Lerp(Vector) (Variables|Default|GetStartLocation) (+ (Variables|Default|GetStartLocation) (* (Transformation|GetActorForwardVector) (Variables|Default|Getdistance))) _newtrack_0) false false))
    (:Finished
      (Utilities|FlowControl|Delay 0.1)
      (Timeline|Timeline ReverseFromEnd))))

(event Collision|EventActorBeginOverlap
  (params (OtherActor :type Actor%20Object%20Reference)))

(event EventTick
  (params (DeltaSeconds :type Float%20%28single-precision%29)))

(fn ConstructionScript)